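; Demo actor that builds a triangulated mesh from multiple outer contours with holes cut into it.
; The BuildTriangulatedMesh event clears all sections on TriangulateDemo, then calls CreateMeshWithHoles on it.
; Two outer contours and two holes are each converted through MakeTriangulateContour and passed as the outer and inner contour arrays.
; The construction script is empty and BeginPlay, overlap and Tick are disabled, so nothing here triggers the build automatically.
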(event `BuildTriangulatedMesh`
  (`ProceduralMeshComponent.ClearAllMeshSections` (`self.TriangulateDemo`))
  (`TriangulateDemoComponent.CreateMeshWithHoles` (`self.TriangulateDemo`) (`|MakeArray` (`TriangulateFunctionLibrary.MakeTriangulateContour` (`self.Contour1`)) (`TriangulateFunctionLibrary.MakeTriangulateContour` (`self.Contour2`))) (`|MakeArray` (`TriangulateFunctionLibrary.MakeTriangulateContour` (`self.Hole1`)) (`TriangulateFunctionLibrary.MakeTriangulateContour` (`self.Hole2`)))))

(fn `UserConstructionScript`)